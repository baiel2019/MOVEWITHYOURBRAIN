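; Platform actor that starts moving between its position and an offset (MoveToPas) when its IsPressed event fires.
; IsPressed stores the start location and enables Tick, which accumulates delta time scaled by the Time variable.
; Tick scrubs a Timeline to the wrapped value instead of playing it, and the Timeline's update lerps the actor's location without sweep.
; An InterpToMovement control-point setup is left disconnected.
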(event `self.ReceiveActorBeginOverlap`
  (params (OtherActor :type "Actor Object Reference")))

(event `/Game/log/I_butten.isPressed`
  (set `self.start location` (`self.K2_GetActorLocation`))
  (`self.SetActorTickEnabled` true))

(event `self.ReceiveTick`
  (params (DeltaSeconds :type "Float (single-precision)"))
  (bind _start_location (`self.start location`))
  (bind _output_get (set `self.alpha` (+ (/ DeltaSeconds (`self.time`)) (`self.alpha`))))
  (bind (_direction _alpha) (`Timeline|Timeline` :`NewTime` (mod _output_get 1.0) :!via `SetNewTime`)
    (:`Update`
      (`self.K2_SetActorLocation` (`KismetMathLibrary.VLerp` _start_location (+ _start_location (`self.MoveToPas`)) _alpha)))))

(fn `AddIKGoals`
  (returns (OutGoals :type "Map of Name to IKRigGoal Structure"))
  (return))

(fn `UserConstructionScript`)