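; BP_movable is a physics prop that takes a table, chair, board or cube mesh by type and can be dragged around.
; A move event creates or repositions a breakable physics constraint linking a sphere to the simulated mesh, and an end event destroys it.
; Tick respawns the mesh above its starting point with zero velocity if it falls too far below the world.
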(event `location sphere`
  (params (NewParam :type "Vector Structure"))
  (bind _physics_constraint (`self.Physics Constraint`))
  (bind _physics_constraint_2 (`self.Physics Constraint`))
  ;[1 1 1] give up
  (`/Engine/EditorBlueprintResources/StandardMacros.IsValid` _physics_constraint_2
    (:`Is Valid`
      (`SceneComponent.K2_SetWorldLocation` _physics_constraint_2 NewParam false false))
    (:`Is Not Valid`
      (bind _returnvalue (`AddComponent|NODE_AddPhysicsConstraintComponent-0` :`RelativeTransform` (`KismetMathLibrary.MakeTransform` (- NewParam (`self.K2_GetActorLocation`)))))
      (bind _output_get (set `self.Physics Constraint` _returnvalue))
      (`SceneComponent.K2_AttachToComponent` (`self.Sphere`) _output_get "None" "KeepRelative" "KeepRelative" "KeepRelative" true)
      (`PhysicsConstraintComponent.SetConstrainedComponents` (`self.Physics Constraint`) (`self.Sphere`) "None" (`self.StaticMesh`) "None")
      (`ActorComponent.SetActive` (`self.Physics Constraint`) true false)
      (`PhysicsConstraintComponent.SetLinearBreakable` _physics_constraint true 49500000.0)
      (`ActorComponent.SetTickGroup` _physics_constraint "TG_PrePhysics"))))

(event `self.ReceiveTick`
  (params (DeltaSeconds :type "Float (single-precision)"))
  (bind _staticmesh (`self.StaticMesh`))
  ;[1 1 1] return
  (if (< (.z (`SceneComponent.K2_GetComponentLocation` (`self.StaticMesh`))) -3000.0)
    (`SceneComponent.K2_SetWorldLocation` _staticmesh (+ (`self.starting locate`) (`KismetMathLibrary.MakeVector` 0.0 0.0 1000.0)) false false)
    (`PrimitiveComponent.SetPhysicsLinearVelocity` _staticmesh (0.0 0.0 0.0) false "None")))

(event `end move`
  ;[1 1 1] end move
  (`ActorComponent.K2_DestroyComponent` (`self.Physics Constraint`))
  (set `self.Physics Constraint` null))

(event `self.ReceiveBeginPlay`
  (bind _staticmesh (`self.StaticMesh`))
  ;[1 1 1] locate
  (set `self.starting locate` (`SceneComponent.K2_GetComponentLocation` (`self.StaticMesh`)))
  (switch `/Game/log/E_movableType` (`self.Type of object`)
    (:`NewEnumerator0`
      (`StaticMeshComponent.SetStaticMesh` (`self.StaticMesh`) "/Game/StarterContent/Props/object/boardone_Plane.boardone_Plane"))
    (:`NewEnumerator1`
      (`StaticMeshComponent.SetStaticMesh` (`self.StaticMesh`) "/Game/StarterContent/Props/object/chairone.chairone"))
    (:`NewEnumerator2`
      (`StaticMeshComponent.SetStaticMesh` (`self.StaticMesh`) "/Game/StarterContent/Props/object/board.board"))
    (:`NewEnumerator3`
      (`StaticMeshComponent.SetStaticMesh` (`self.StaticMesh`) "/Game/StarterContent/Shapes/Shape_Cube.Shape_Cube")))
  (`PrimitiveComponent.SetSimulatePhysics` _staticmesh true)
  (`PrimitiveComponent.SetMassOverrideInKg` _staticmesh "None" 300.0 true))

(fn `UserConstructionScript`)